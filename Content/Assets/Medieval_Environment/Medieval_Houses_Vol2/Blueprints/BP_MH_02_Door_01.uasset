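; BP_MH_02_Door_01 is an interactable hinged door for the medieval house set, with three selectable wooden door meshes.
; The construction script clamps DoorType to pick the mesh and sizes a detection sphere from DetectionRadius.
; StartLook and EndLook toggle custom depth on the door for highlighting.
; StartInterack flips the Closed state, playing or reversing a timeline that swings the door's yaw open or shut.
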(event Custom|StartMove
  (bind _rotationcoeff (Timeline|Timeline_Rotation Play)
    (:Update
      (Transformation|SetRelativeRotation (Variables|Default|GetDoor_Left) (Math|Rotator|MakeRotator 0.0 0.0 (* _rotationcoeff 92.0)) false false))))

(event Custom|StartUnmove
  (bind _rotationcoeff (Timeline|Timeline_Rotation Reverse)
    (:Update
      (Transformation|SetRelativeRotation (Variables|Default|GetDoor_Left) (Math|Rotator|MakeRotator 0.0 0.0 (* _rotationcoeff 92.0)) false false))))

(fn ConstructionScript
  (Components|Sphere|SetSphereRadius (Variables|Default|GetSphere) (Variables|Default|GetDetectionRadius) true)
  (bind _output_get (Variables|Default|SetDoorType (Math|Integer|Clamp(Integer) (Variables|Default|GetDoorType) 0 2)))
  (switch int _output_get
    (:0
      (Components|StaticMesh|SetStaticMesh (Variables|Default|GetDoor_Left) "/Game/Assets/Medieval_Environment/Medieval_Houses_Vol2/Meshes/SM_MH_02_Wood_Door_01.SM_MH_02_Wood_Door_01"))
    (:1
      (Components|StaticMesh|SetStaticMesh (Variables|Default|GetDoor_Left) "/Game/Assets/Medieval_Environment/Medieval_Houses_Vol2/Meshes/SM_MH_02_Wood_Door_02.SM_MH_02_Wood_Door_02"))
    (:2
      (Components|StaticMesh|SetStaticMesh (Variables|Default|GetDoor_Left) "/Game/Assets/Medieval_Environment/Medieval_Houses_Vol2/Meshes/SM_MH_02_Wood_Door_03.SM_MH_02_Wood_Door_03"))))

(fn EndLook
  (params (Actor :type Actor%20Object%20Reference))
  (Rendering|SetRenderCustomDepth (Variables|Default|GetDoor_Left) false)
  (return false))

(fn StartInterack
  (params (Actor :type Actor%20Object%20Reference))
  (if (Variables|Default|GetClosed)
    (CallFunction|StartMove)
    (Variables|Default|SetClosed false)
    (else
      (CallFunction|StartUnmove)
      (Variables|Default|SetClosed true)))
  (return false))

(fn StartLook
  (params (Actor :type Actor%20Object%20Reference))
  (Rendering|SetRenderCustomDepth (Variables|Default|GetDoor_Left) true)
  (return false))